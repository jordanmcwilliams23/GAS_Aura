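; Base enemy character Blueprint providing spawn, dissolve, loot-drop and champion split behavior.
; Timelines scale the mesh on spawn and fade enemy and weapon dissolve materials, while Motion Warping receives the facing target.
; Loot from loot tiers spawns one item per looping timer tick, ringed around the enemy.
; Split marks an arc with summon effects, then spawns scaled, non-champion clones of its own class one by one, facing the combat target.
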(event `self.ReceiveBeginPlay`
  ;[1 1 1] Spawn
  (`parent.ReceiveBeginPlay`)
  (`|ExecutionSequence`
    (:`then_0`
      (bind _spawnsound (`self.SpawnSound`)
        (:`then`
          (`GameplayStatics.PlaySoundAtLocation` _spawnsound (`self.K2_GetActorLocation`) (struct) 1.0 1.0 0.0 null null null null))
        (:`else`)))
    (:`then_1`
      (bind (_direction _scaletrack) (`Timeline|Spawn Timeline`)
        (:`Update`
          (`SceneComponent.SetRelativeScale3D` (`self.Mesh`) (`KismetMathLibrary.MakeVector` _scaletrack _scaletrack _scaletrack)))))))

(event `self.StartDissolveTimeline`
  (params (EnemyDissolveDMI :type "MaterialInstanceDynamic Object Reference") (WeaponDissolveDMI :type "MaterialInstanceDynamic Object Reference"))
  ;[1 0.4634 0.3027] Dissolve
  (bind (_direction _dissolve_track) (`Timeline|Dissolve Timeline`)
    (:`Update`
      (`MaterialInstanceDynamic.SetScalarParameterValue` WeaponDissolveDMI "Dissolve" _dissolve_track)
      (`MaterialInstanceDynamic.SetScalarParameterValue` EnemyDissolveDMI "Dissolve" _dissolve_track))))

(event `CombatInterface.SetFacingTarget`
  (params (TargetLocation :type "Vector Structure"))
  ;[1 0.7896 0.2993] Set Facing Target
  (`MotionWarpingComponent.AddOrUpdateWarpTargetFromLocation` (`self.MotionWarping`) "FacingTarget" TargetLocation))

(event `self.SpawnLoot`
  (bind _returnvalue (`AuraAbilitySystemLibrary.GetLootTiers` null))
  ;[1 1 1] Spawn Loot
  (`/Engine/EditorBlueprintResources/StandardMacros.IsValid` _returnvalue
    (:`Is Valid`
      (bind _output_get (set `self.Loot Items` (`LootTiers.GetLootItems` _returnvalue self)))
      (set `self.LootRotations` (`self.GetLootRotations` _output_get))
      (set `self.SpawnLootCount` 0)
      (bind _returnvalue_2 (`KismetSystemLibrary.K2_SetTimer` null "SpawnLootItem" 0.12 true))
      (set `self.SpawnLootTimerHandle` _returnvalue_2))))

(event `self.Split`
  (params (DeadCharacter :type "Actor Object Reference"))
  (bind (_returnvalue_bchampionsenabled _returnvalue_championattributemultiplierrange _returnvalue_scalemultiplier _returnvalue_extranumlootitems _returnvalue_extraspawnlootchance _returnvalue_regenerator_healthpercentthreshold _returnvalue_regenerator_regenduration _returnvalue_regenerator_regenperiod _returnvalue_regenerator_regenpercent _returnvalue_regenerationgameplayeffectclass _returnvalue_shooter_firerate _returnvalue_shooter_fireprojectileclass _returnvalue_speedy_speedmultiplier _returnvalue_splitter_numsplitinto _returnvalue_splitter_spawndistance) (break `ChampionInformation` (`AuraAbilitySystemLibrary.GetChampionInfo` null)))
  (bind (_returnvalue_bchampionsenabled_2 _returnvalue_championattributemultiplierrange_2 _returnvalue_scalemultiplier_2 _returnvalue_extranumlootitems_2 _returnvalue_extraspawnlootchance_2 _returnvalue_regenerator_healthpercentthreshold_2 _returnvalue_regenerator_regenduration_2 _returnvalue_regenerator_regenperiod_2 _returnvalue_regenerator_regenpercent_2 _returnvalue_regenerationgameplayeffectclass_2 _returnvalue_shooter_firerate_2 _returnvalue_shooter_fireprojectileclass_2 _returnvalue_speedy_speedmultiplier_2 _returnvalue_splitter_numsplitinto_2 _returnvalue_splitter_spawndistance_2 _returnvalue_splitter_clonescalemultiplier) (break `ChampionInformation` (`AuraAbilitySystemLibrary.GetChampionInfo` null)))
  (bind _output (`|GetArrayItem` (`self.SpawnLocations`) (`self.SpawnIndex`)))
  (`GameplayStatics.PlaySoundAtLocation` "/Game/Assets/Sounds/Enemies/Demon/Death/sfx_Ghoul_Death.sfx_Ghoul_Death" (`self.K2_GetActorLocation`) (struct) 1.0 1.0 0.0 null null null null)
  (set `self.SpawnIndex` 0)
  (bind _output_get (set `self.SpawnDirections` (`AuraAbilitySystemLibrary.EvenlyRotatedVectors` (`self.GetActorForwardVector`) (`KismetMathLibrary.Vector_Up`) 270.0 (`KismetMathLibrary.Conv_ByteToInt` _returnvalue_splitter_numsplitinto))))
  (for _array_element _output_get
    (`KismetArrayLibrary.Array_Add` (`self.SpawnLocations`) (+ (`self.K2_GetActorLocation`) (* _array_element _returnvalue_splitter_spawndistance))))
  (for _array_element_2 (`self.SpawnLocations`)
    (`NiagaraFunctionLibrary.SpawnSystemAtLocation` "/Game/Assets/Effects/Combat/NS_GroundSummon.NS_GroundSummon" (+ _array_element_2 (`KismetMathLibrary.MakeVector` 0.0 0.0 (* (`CapsuleComponent.GetScaledCapsuleHalfHeight` (`self.CapsuleComponent`)) -1.0)))))
  (if (`KismetArrayLibrary.Array_IsValidIndex` (`self.SpawnLocations`) (`self.SpawnIndex`)) :!label _label
    (`KismetSystemLibrary.Delay` 1.0)
    (bind _returnvalue (`|SpawnActorFromClass` (`GameplayStatics.GetObjectClass` self) (`KismetMathLibrary.MakeTransform` _output (`KismetMathLibrary.FindLookAtRotation` _output (`self.K2_GetActorLocation` (`TargetInterface.GetCombatTarget`))) (`KismetMathLibrary.Conv_DoubleToVector` _returnvalue_splitter_clonescalemultiplier)) "AdjustIfPossibleButAlwaysSpawn" "MultiplyWithRoot" null (`self.Level`) false null))
    (`self.SpawnDefaultController` _returnvalue)
    (`/Engine/EditorBlueprintResources/StandardMacros.IncrementInt` (`self.SpawnIndex`)
      (:`  `
        (goto _label)))))

(fn `GetLootRotations`
  (params (TargetArray :type "Array of LootItem Structure (by ref)"))
  (returns (ReturnValue :type "Array of Rotator Structure"))
  (return (`AuraAbilitySystemLibrary.EvenlySpacedRotators` (`self.GetActorForwardVector`) (`KismetMathLibrary.Vector_Up`) 360.0 (`KismetArrayLibrary.Array_Length` TargetArray))))

(fn `GetLootTransform`
  (returns (`Spawn Transform` :type "Transform Structure"))
  (bind _output (`|GetArrayItem` (`self.LootRotations`) (`self.SpawnLootCount`)))
  (return (`KismetMathLibrary.MakeTransform` (+ (`self.K2_GetActorLocation`) (* (`KismetMathLibrary.GetForwardVector` _output) (`KismetMathLibrary.RandomFloatInRange` (`self.SpawnLootDistanceMin`) (`self.SpawnLootDistanceMax`)))) _output)))

(fn `SpawnLootItem`
  (locals (CurrentLootItem :type "LootItem Structure"))
  (if (`KismetArrayLibrary.Array_IsValidIndex` (`self.Loot Items`) (`self.SpawnLootCount`))
    (bind _output_get (set `local.CurrentLootItem` (`|GetArrayItem` (`self.Loot Items`) (`self.SpawnLootCount`))))
    (`|SpawnActorFromClass` (break `LootItem` _output_get) (`self.GetLootTransform`) "AdjustIfPossibleButAlwaysSpawn" "MultiplyWithRoot" null (`KismetMathLibrary.SelectInt` (`self.Level`) 1 (`.bLootLevelOverride` (break `LootItem` _output_get))) null)
    (`/Engine/EditorBlueprintResources/StandardMacros.IncrementInt` (`self.SpawnLootCount`))
    (else
      (`KismetSystemLibrary.K2_ClearAndInvalidateTimerHandle` (`self.SpawnLootTimerHandle`)))))

(fn `UserConstructionScript`)