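; BP_AuraMainMenu is the main menu scene actor that sets up the menu view, music and UI.
; On BeginPlay it blends the view to MainCamera, starts menu music and creates WBP_MainMenu with that audio component, switching to UI-only input with a visible cursor.
; Each Tick bobs the Fireball component vertically around its starting position using a wrapped sine timer.
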(event `self.ReceiveBeginPlay`
  (`PlayerController.SetViewTargetWithBlend` (`GameplayStatics.GetPlayerController` 0) (`self.MainCamera`) 0.0 "VTBlend_Linear" 0.0 false)
  (set `self.FireballStartingPosition` (`SceneComponent.K2_GetComponentLocation` (`self.Fireball`)))
  (bind _returnvalue (`GameplayStatics.SpawnSound2D` "/Game/Assets/Sounds/Music/Music_MainMenu.Music_MainMenu" 1.0 1.0 0.0 null))
  (bind _output_get (set `self.MusicAudioComponent` _returnvalue))
  (bind _returnvalue_2 (`|CreateWidget` "/Game/Blueprints/UI/MainMenu/WBP_MainMenu.WBP_MainMenu_C" null _output_get))
  (`UserWidget.AddToViewport` _returnvalue_2 0)
  (`WidgetBlueprintLibrary.SetInputMode_UIOnlyEx` (`GameplayStatics.GetPlayerController` 0) _returnvalue_2)
  (set `PlayerController.bShowMouseCursor` true (`GameplayStatics.GetPlayerController` 0)))

(event `self.ReceiveTick`
  (params (DeltaSeconds :type "Float (single-precision)"))
  (bind _output_get (set `self.Time` (+ (stale _output_get) DeltaSeconds)))
  (if (> _output_get 6.28318)
    (bind _output_get_2 (set `self.Time` 0.0)))
  (`SceneComponent.K2_SetWorldLocation` (`self.Fireball`) (+ (`self.FireballStartingPosition`) (`KismetMathLibrary.MakeVector` 0.0 0.0 (* (`KismetMathLibrary.Sin` _output_get_2) (`self.FireballHoverMagnitude`)))) false false))

(fn `UserConstructionScript`)