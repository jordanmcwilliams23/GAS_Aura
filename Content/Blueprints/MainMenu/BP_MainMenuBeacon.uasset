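; BP_MainMenuBeacon is a main menu beacon actor whose glow pulses continuously.
; BeginPlay creates a dynamic material instance on the beacon mesh.
; Each Tick advances a timer that wraps after one sine period and drives the material's Glow parameter with a sine wave, scaled by a glow multiplier and offset by a minimum brightness.
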(event `self.ReceiveBeginPlay`
  (bind _returnvalue (`PrimitiveComponent.CreateDynamicMaterialInstance` (`self.BeaconMesh`) 0 null "None"))
  (set `self.BeaconDMI` _returnvalue))

(event `self.ReceiveTick`
  (params (DeltaSeconds :type "Float (single-precision)"))
  (bind _output_get (set `self.Time` (+ (stale _output_get) DeltaSeconds)))
  (if (> _output_get 6.28)
    (bind _output_get_2 (set `self.Time` 0.0)))
  (`MaterialInstanceDynamic.SetScalarParameterValue` (`self.BeaconDMI`) "Glow" (+ (* (`KismetMathLibrary.Sin` _output_get_2) (`self.GlowMultiplier`)) (`self.Minimum Brightness`))))

(fn `UserConstructionScript`)