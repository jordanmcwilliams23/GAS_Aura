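; Enemy ranged attack gameplay ability that turns its avatar toward its combat target and fires a projectile at it.
; It plays a random tagged attack montage, waits once for that montage's event tag, then spawns the projectile from the matching socket tag.
; The aim point is the target's location at activation, raised by the square root of the distance when fired.
; The ability ends when the montage completes, is interrupted or is cancelled.
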(event `self.K2_ActivateAbility`
  (bind _returnvalue (`self.GetAvatarActorFromActorInfo`))
  (bind (_taggedmontage_montage _taggedmontage_montagetag _taggedmontage_sockettag) (break `TaggedMontage` (`self.TaggedMontage`)))
  (bind _returnvalue_2 (message `TargetInterface.GetCombatTarget` _returnvalue))
  (bind _output_get (set `self.Combat Target` _returnvalue_2))
  (bind _output_get_2 (set `self.TargetLocation` (`Actor.K2_GetActorLocation` _output_get)))
  (message `CombatInterface.SetFacingTarget` _returnvalue _output_get_2)
  (bind _returnvalue_3 (message `CombatInterface.GetAttackMontages` _returnvalue))
  (bind _output_get_3 (set `self.TaggedMontage` (`KismetArrayLibrary.Array_Random` _returnvalue_3)))
  (bind (_montage _montagetag) (break `TaggedMontage` _output_get_3))
  (`AbilityTask_PlayMontageAndWait.CreatePlayMontageAndWaitProxy` "None" _montage
    (:`then`
      (`AbilityTask_WaitGameplayEvent.WaitGameplayEvent` _montagetag null true
        (:`EventReceived`
          (`self.SpawnProjectile` _taggedmontage_sockettag (+ (`self.TargetLocation`) (`KismetMathLibrary.MakeVector` 0.0 0.0 (`KismetMathLibrary.Sqrt` (`Actor.GetDistanceTo` (`self.GetAvatarActorFromActorInfo`) (`self.Combat Target`)))))))))
    (:`OnCompleted`
      (`self.K2_EndAbility` :!label _label))
    (:`OnInterrupted`
      (goto _label))
    (:`OnCancelled`
      (goto _label))))