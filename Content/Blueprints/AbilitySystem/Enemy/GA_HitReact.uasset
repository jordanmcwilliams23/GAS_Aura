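; Enemy gameplay ability that plays a hit reaction montage while GE_HitReact is applied to its owner.
; It gets the montage and crowd control (CC) stack count from the avatar through message calls, scales play rate by that count and CCPlayRateMult, then adds a stack.
; The ability ends when the montage finishes, is interrupted or cancelled, or is missing, removing the effect and ending the montage task.
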(event `self.K2_ActivateAbility`
  (bind _returnvalue (`self.GetAvatarActorFromActorInfo`))
  (bind _returnvalue_2 (`self.BP_ApplyGameplayEffectToOwner` "/Game/Blueprints/AbilitySystem/GameplayEffects/GE_HitReact.GE_HitReact_C"))
  (set `self.HitReactEffectHandle` _returnvalue_2)
  (bind _returnvalue_3 (message `CombatInterface.GetHitReactMontage` _returnvalue))
  (`/Engine/EditorBlueprintResources/StandardMacros.IsValid` _returnvalue_3
    (:`Is Valid`
      (bind _returnvalue_4 (message `CombatInterface.GetCCStacks` _returnvalue))
      (bind _asynctaskproxy (`AbilityTask_PlayMontageAndWait.CreatePlayMontageAndWaitProxy` "None" _returnvalue_3 (+ 1.0 (* _returnvalue_4 (`self.CCPlayRateMult`))))
        (:`then`
          (set `self.Montage Async Task` _asynctaskproxy)
          (message `CombatInterface.AddCCStacks` (`self.GetAvatarActorFromActorInfo`) 1))
        (:`OnCompleted`
          (`self.K2_EndAbility` :!label _label))
        (:`OnInterrupted`
          (goto _label))
        (:`OnCancelled`
          (goto _label))))
    (:`Is Not Valid`
      (goto _label))))

(event `self.K2_OnEndAbility`
  (params (bWasCancelled :type Boolean))
  (`self.BP_RemoveGameplayEffectFromOwnerWithHandle` (`self.HitReactEffectHandle`))
  (bind _montage_async_task (`self.Montage Async Task`)
    (:`then`
      (`GameplayTask.EndTask` _montage_async_task))
    (:`else`)))