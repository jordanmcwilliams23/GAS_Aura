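; Enemy melee attack Gameplay Ability that faces the combat target and deals area damage to live players.
; It plays a random attack montage from the avatar and waits once for that montage's tagged gameplay event.
; On the event it checks a radius around the montage's combat socket, damages non-friendly players, and fires a melee impact cue if anything was hit.
; The ability ends when the montage completes, is interrupted or is cancelled, and can draw a debug sphere.
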(event `self.K2_ActivateAbility`
  (bind _returnvalue (`self.GetAvatarActorFromActorInfo`))
  (bind _returnvalue_2 (`self.GetAvatarActorFromActorInfo`))
  (bind (_taggedmontage_montage _taggedmontage_montagetag) (break `TaggedMontage` (`self.TaggedMontage`)))
  (set `self.HasHitTarget` false)
  (bind _returnvalue_3 (message `TargetInterface.GetCombatTarget` _returnvalue_2))
  (bind _output_get (set `self.CombatTarget` _returnvalue_3))
  (message `CombatInterface.SetFacingTarget` _returnvalue_2 (`Actor.K2_GetActorLocation` _output_get))
  (bind _returnvalue_4 (message `CombatInterface.GetAttackMontages` _returnvalue_2))
  (bind _output_get_2 (set `self.TaggedMontage` (`KismetArrayLibrary.Array_Random` _returnvalue_4)))
  (bind (_montage _montagetag _sockettag) (break `TaggedMontage` _output_get_2))
  (`AbilityTask_PlayMontageAndWait.CreatePlayMontageAndWaitProxy` "None" _montage
    (:`then`
      (`AbilityTask_WaitGameplayEvent.WaitGameplayEvent` _montagetag null true
        (:`EventReceived`
          (bind _returnvalue_5 (message `CombatInterface.GetCombatSocketLocation` _returnvalue _sockettag))
          (set `self.CombatSocketLocation` _returnvalue_5)
          (bind _outoverlappingactors (`AuraAbilitySystemLibrary.GetLivePlayersWithinRadius` _returnvalue (`|MakeArray` _returnvalue) (`self.AttackRadius`) (`self.CombatSocketLocation`)))
          (for _array_element _outoverlappingactors
            (if (`AuraAbilitySystemLibrary.IsNotFriend` (`self.GetAvatarActorFromActorInfo`) _array_element)
              (`AuraAbilitySystemLibrary.ApplyDamageEffect` (`self.MakeDamageEffectParamsFromEffectDefaults` _array_element))
              (set `self.HasHitTarget` true)))
          (if (`self.HasHitTarget`)
            (`self.K2_ExecuteGameplayCueWithParams` (struct :`TagName` "GameplayCue.MeleeImpact") (`AbilitySystemBlueprintLibrary.MakeGameplayCueParameters` 0.0 0.0 (struct) (struct) (struct) (`BlueprintGameplayTagLibrary.MakeGameplayTagContainerFromTag` _taggedmontage_montagetag) (struct) (`self.CombatSocketLocation`) (0.0 0.0 0.0) null null (`self.CombatTarget`))))
          (if (`self.DrawDebugSphere?`)
            (`KismetSystemLibrary.DrawDebugSphere` (`self.CombatSocketLocation`) (`self.AttackRadius`) 12 (struct :`R` 1.0 :`B` 0.044127 :`A` 1.0) 2.0 2.0)))))
    (:`OnCompleted`
      (`self.K2_EndAbility` :!label _label))
    (:`OnInterrupted`
      (goto _label))
    (:`OnCancelled`
      (goto _label))))