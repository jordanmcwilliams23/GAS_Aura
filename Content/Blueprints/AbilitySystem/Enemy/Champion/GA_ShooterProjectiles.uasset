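; Gameplay ability for Champion enemies with the Shooter behavior that repeatedly fires homing projectiles at the combat target.
; On activation, a looping timer runs at the fire rate from the character class info's Champion data.
; Each shot spawns at a randomized offset from the avatar, using an elliptical cone around its forward vector, with a pitch override.
; The ability ends when a tick finds the avatar or target dead, and ending clears the timer.
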(event `self.K2_ActivateAbility`
  (bind (_championinfo_bchampionsenabled _championinfo_championattributemultiplierrange _championinfo_scalemultiplier _championinfo_extranumlootitems _championinfo_extraspawnlootchance _championinfo_experiencemultiplier _championinfo_regenerator_healthpercentthreshold _championinfo_regenerator_regenduration _championinfo_regenerator_regenperiod _championinfo_regenerator_regenpercent _championinfo_regenerationgameplayeffectclass _championinfo_shooter_firerate) (break `ChampionInformation` (`CharacterClassInfo.ChampionInfo` (`AuraAbilitySystemLibrary.GetCharacterClassInfo` null))))
  (set `self.AvatarActor` (`self.GetAvatarActorFromActorInfo`))
  (bind _output_get (set `self.FireProjectileRate` _championinfo_shooter_firerate))
  (bind _returnvalue (`KismetSystemLibrary.K2_SetTimerDelegate` (delegate `FireProjectile`) _output_get true))
  (set `self.FireProjectileTimerHandle` _returnvalue))

(event `FireProjectile`
  (bind _returnvalue (message `CombatInterface.IsDead` (`self.AvatarActor`)))
  (if _returnvalue
    (`self.K2_EndAbility`)
    (else
      (bind _returnvalue_2 (message `TargetInterface.GetCombatTarget` (`self.AvatarActor`)))
      (set `self.CombatTarget` _returnvalue_2)
      (bind _combattarget (`self.CombatTarget`)
        (:`then`
          (bind _returnvalue_3 (message `CombatInterface.IsDead` _combattarget))
          (if _returnvalue_3
            (`self.K2_EndAbility`)
            (else
              (bind _output_get (set `self.ProjectileTargetLocation` (`Actor.K2_GetActorLocation` (`self.CombatTarget`))))
              (`self.SpawnProjectiles` _output_get (`BlueprintGameplayTagLibrary.MakeLiteralGameplayTag` (struct)) (`self.CombatTarget`) 30.0 (+ (`Actor.K2_GetActorLocation` (`self.GetAvatarActorFromActorInfo`)) (* (`self.ProjectileSpawnDistance`) (`KismetMathLibrary.RandomUnitVectorInEllipticalConeInRadians` (`Actor.GetActorForwardVector` (`self.GetAvatarActorFromActorInfo`)) 90.0 1.0)))))))
        (:`else`)))))

(event `self.K2_OnEndAbility`
  (params (bWasCancelled :type Boolean))
  (`KismetSystemLibrary.K2_ClearAndInvalidateTimerHandle` (`self.FireProjectileTimerHandle`)))