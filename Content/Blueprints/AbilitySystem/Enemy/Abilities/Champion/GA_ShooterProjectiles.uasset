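; Gameplay ability for the Shooter champion enemy that repeatedly fires projectiles at its combat target.
; On activation it starts a looping timer at the fire rate from the champion class info.
; Each tick spawns projectiles at a random offset within a wide, nearly flat forward cone, with a pitch override and the target set for homing.
; When the target is dead, it clears the timer and ends the ability.
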(event `self.K2_ActivateAbility`
  (bind (_championinfo_bchampionsenabled _championinfo_championattributemultiplierrange _championinfo_scalemultiplier _championinfo_extranumlootitems _championinfo_extraspawnlootchance _championinfo_regenerator_healthpercentthreshold _championinfo_regenerator_regenduration _championinfo_regenerator_regenperiod _championinfo_regenerator_regenpercent _championinfo_regenerationgameplayeffectclass _championinfo_shooter_firerate) (break `ChampionInfo` (`CharacterClassInfo.ChampionInfo` (`AuraAbilitySystemLibrary.GetCharacterClassInfo` null))))
  (bind _output_get (set `self.FireProjectileRate` _championinfo_shooter_firerate))
  (bind _returnvalue (`KismetSystemLibrary.K2_SetTimerDelegate` (delegate `FireProjectile`) _output_get true))
  (set `self.FireProjectileTimerHandle` _returnvalue))

(event `FireProjectile`
  (bind _returnvalue (message `TargetInterface.GetCombatTarget` (`self.GetAvatarActorFromActorInfo`)))
  (`/Engine/EditorBlueprintResources/StandardMacros.IsValid` _returnvalue
    (:`Is Valid`
      (bind _output_get (set `self.CombatTarget` _returnvalue))
      (bind _returnvalue_2 (message `CombatInterface.IsDead` _output_get))
      (if _returnvalue_2
        (`KismetSystemLibrary.K2_ClearAndInvalidateTimerHandle` (`self.FireProjectileTimerHandle`))
        (`self.K2_EndAbility`)
        (else
          (bind _output_get_2 (set `self.ProjectileTargetLocation` (`Actor.K2_GetActorLocation` (`self.CombatTarget`))))
          (`self.SpawnProjectiles` _output_get_2 (`BlueprintGameplayTagLibrary.MakeLiteralGameplayTag` (struct)) (`self.CombatTarget`) 30.0 (+ (`Actor.K2_GetActorLocation` (`self.GetAvatarActorFromActorInfo`)) (* (`self.ProjectileSpawnDistance`) (`KismetMathLibrary.RandomUnitVectorInEllipticalConeInRadians` (`Actor.GetActorForwardVector` (`self.GetAvatarActorFromActorInfo`)) 90.0 1.0)))))))))