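; Enemy gameplay ability that summons random minions at shuffled spawn locations around the avatar's logic-provided points.
; On activation it plays a ground summon effect at every location and runs the avatar's summon montage.
; An Abilities.Summon gameplay event starts a delayed loop that spawns minions one by one, facing away from the summoner, with default controllers.
; Each spawn increments the avatar's minion count, and its bound death event decrements it.
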(event `self.K2_ActivateAbility`
  (bind _returnvalue (`self.GetRandomMinionCDO`))
  (bind _spawnlocations (`self.SpawnLocations`))
  (bind _returnvalue_2 (+ (`|GetArrayItem` _spawnlocations (`self.SpawnLocationIndex`)) (`KismetMathLibrary.MakeVector` 0.0 0.0 (`CapsuleComponent.GetScaledCapsuleHalfHeight` (`Character.CapsuleComponent` _returnvalue)))))
  (set `self.SpawnLocationIndex` 0)
  (set `self.AvatarActor` (`self.GetAvatarActorFromActorInfo`))
  (bind _output_get (set `self.SpawnLocations` (`self.GetSpawnLocations`)))
  (`KismetArrayLibrary.Array_Shuffle` _output_get)
  (for _array_element (`self.SpawnLocations`)
    (`NiagaraFunctionLibrary.SpawnSystemAtLocation` "/Game/Assets/Effects/Combat/NS_GroundSummon.NS_GroundSummon" _array_element))
  (bind _returnvalue_3 (message `CombatInterface.GetSummonMontage` (`self.GetAvatarActorFromActorInfo`)))
  (`AbilityTask_PlayMontageAndWait.CreatePlayMontageAndWaitProxy` "None" _returnvalue_3
    (:`then`
      (`AbilityTask_WaitGameplayEvent.WaitGameplayEvent` (struct :`TagName` "Abilities.Summon") null
        (:`EventReceived`
          (if (< (`self.SpawnLocationIndex`) (`KismetArrayLibrary.Array_Length` _spawnlocations)) :!label _label
            (bind _returnvalue_4 (`|SpawnActorFromClass` (`GameplayStatics.GetObjectClass` _returnvalue) (`KismetMathLibrary.MakeTransform` _returnvalue_2 (`KismetMathLibrary.FindLookAtRotation` (`Actor.K2_GetActorLocation` (`self.GetAvatarActorFromActorInfo`)) _returnvalue_2)) "AlwaysSpawn" "MultiplyWithRoot" null null))
            (add `AuraCharacterBase.OnDeath` _returnvalue_4 (delegate `CharacterDied_Event`))
            (message `CombatInterface.IncrementMinionCount` (`self.AvatarActor`) 1)
            (`Pawn.SpawnDefaultController` _returnvalue_4)
            (`/Engine/EditorBlueprintResources/StandardMacros.IncrementInt` (`self.SpawnLocationIndex`)
              (:`  `
                (`KismetSystemLibrary.Delay` 0.2)
                (goto _label)))))))))

(event `CharacterDied_Event`
  (params (DeadCharacter :type "Actor Object Reference"))
  (message `CombatInterface.IncrementMinionCount` (`self.AvatarActor`) -1))