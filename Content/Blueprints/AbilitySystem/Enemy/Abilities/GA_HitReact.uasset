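; GA_HitReact is an enemy gameplay ability that plays the avatar's hit reaction.
; On activation it applies GE_HitReact to the owner, stores the handle, and plays the montage the avatar returns from GetHitReactMontage.
; The ability ends when the montage completes, is interrupted or cancelled, or immediately if none is valid.
; Ending removes the effect by its handle and stops the montage task.
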(event `self.K2_ActivateAbility`
  (bind _returnvalue (`self.BP_ApplyGameplayEffectToOwner` "/Game/Blueprints/AbilitySystem/GameplayEffects/GE_HitReact.GE_HitReact_C"))
  (set `self.HitReactEffectHandle` _returnvalue)
  (bind _returnvalue_2 (message `CombatInterface.GetHitReactMontage` (`self.GetAvatarActorFromActorInfo`)))
  (`/Engine/EditorBlueprintResources/StandardMacros.IsValid` _returnvalue_2
    (:`Is Valid`
      (bind _asynctaskproxy (`AbilityTask_PlayMontageAndWait.CreatePlayMontageAndWaitProxy` "None" _returnvalue_2)
        (:`then`
          (set `self.Montage Async Task` _asynctaskproxy))
        (:`OnCompleted`
          (`self.K2_EndAbility` :!label _label))
        (:`OnInterrupted`
          (goto _label))
        (:`OnCancelled`
          (goto _label))))
    (:`Is Not Valid`
      (goto _label))))

(event `self.K2_OnEndAbility`
  (params (bWasCancelled :type Boolean))
  (`self.BP_RemoveGameplayEffectFromOwnerWithHandle` (`self.HitReactEffectHandle`))
  (bind _montage_async_task (`self.Montage Async Task`)
    (:`then`
      (`GameplayTask.EndTask` _montage_async_task))
    (:`else`)))