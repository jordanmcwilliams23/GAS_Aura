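; BP_Firebolt is the Firebolt ability's projectile, adding upkeep for its homing behavior.
; On BeginPlay it starts a looping timer that regularly checks the projectile movement's homing target.
; When that target is invalid or its owner reports dead through the IsDead message, it turns homing off and clears the timer.
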(event `self.ReceiveBeginPlay`
  (bind _returnvalue (`KismetSystemLibrary.K2_SetTimerDelegate` (delegate `CheckValidHomingTarget`) 0.2 true))
  (set `self.CheckHomingTargetHandle` _returnvalue))

(event `CheckValidHomingTarget`
  (bind _homingtargetcomponent (`ProjectileMovementComponent.HomingTargetComponent` (`self.ProjectileMovement`))
    (:`then`
      (bind _returnvalue (message `CombatInterface.IsDead` (`ActorComponent.GetOwner` _homingtargetcomponent)))
      (if _returnvalue
        (set `ProjectileMovementComponent.bIsHomingProjectile` false (`self.ProjectileMovement`) :!label _label)
        (`KismetSystemLibrary.K2_ClearAndInvalidateTimerHandle` (`self.CheckHomingTargetHandle`))))
    (:`else`
      (goto _label))))

(fn `UserConstructionScript`)