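; Firebolt gameplay ability that fires projectiles from the weapon socket toward whatever is under the mouse.
; On activation it commits, captures the cursor's hit location and actor, turns the avatar to face that point and plays the cast montage.
; A montage gameplay event triggers the spawn, passing the hit actor as homing target with a pitch override.
; The ability ends with the montage, and ending it cleans up the target-data task.
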(event `self.K2_ActivateAbility`
  (`self.K2_CommitAbility`)
  (bind (_asynctaskproxy _data) (`TargetDataUnderMouse.CreateTargetDataUnderMouse`)
    (:`then`
      (set `self.TargetDataUnderMouseAsyncTask` _asynctaskproxy))
    (:`ValidDataHandle`
      (bind (_bblockinghit _binitialoverlap _time _distance _location _impactpoint _normal _impactnormal _physmat _hitactor) (`GameplayStatics.BreakHitResult` (`AbilitySystemBlueprintLibrary.GetHitResultFromTargetData` _data)))
      (set `self.ProjectileTargetLocation` _location)
      (set `self.Mouse Hit Actor` _hitactor)
      (message `CombatInterface.SetFacingTarget` (`self.GetAvatarActorFromActorInfo`) (`self.ProjectileTargetLocation`))
      (`AbilityTask_PlayMontageAndWait.CreatePlayMontageAndWaitProxy` "None" "/Game/Assets/Characters/Aura/Animations/Abilities/AM_Cast_FireBolt.AM_Cast_FireBolt" 1.0 "None" false
        (:`then`
          (`AbilityTask_WaitGameplayEvent.WaitGameplayEvent` (struct :`TagName` "Event.Montage.FireBolt") null
            (:`EventReceived`
              (`self.SpawnProjectiles` (`self.ProjectileTargetLocation`) (`BlueprintGameplayTagLibrary.MakeLiteralGameplayTag` (struct :`TagName` "CombatSocket.Weapon")) (`self.Mouse Hit Actor`) 30.0))))
        (:`OnCompleted`
          (`self.K2_EndAbility` :!label _label))
        (:`OnInterrupted`
          (goto _label))
        (:`OnCancelled`
          (goto _label))))))

(event `self.K2_OnEndAbility`
  (params (bWasCancelled :type Boolean))
  (`GameplayTask.EndTask` (`self.TargetDataUnderMouseAsyncTask`)))