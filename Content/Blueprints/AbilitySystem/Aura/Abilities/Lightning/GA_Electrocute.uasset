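; Electrocute gameplay ability: a held lightning beam that shocks the target under the cursor and chains to additional targets.
; On the montage event, the server roots the caster, adds per-target ShockLoop cues and loops a timer that commits cost and applies damage.
; It ends on release after a minimum time, maximum hold, failed cost or death.
; PreEndAbility commits cooldown, clears cues and restores movement, applying a guaranteed stun debuff to targets.
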(event `self.K2_ActivateAbility`
  (`self.EnforceCombatInterface`)
  (bind _asaura_character_base (cast `AuraCharacterBase` (`self.GetAvatarActorFromActorInfo`)))
  (add `AuraCharacterBase.OnDeath` _asaura_character_base (delegate `OnDeath_Event`))
  ;[1 1 1] Store Mouse Data Variables
  (bind (_asynctaskproxy _data) (`TargetDataUnderMouse.CreateTargetDataUnderMouse`)
    (:`ValidDataHandle`
      (`self.StoreMouseDataInfo` (`AbilitySystemBlueprintLibrary.GetHitResultFromTargetData` _data))
      (`self.StoreOwnerVariables`)
      (message `CombatInterface.SetFacingTarget` (`self.GetAvatarActorFromActorInfo`) (`self.MouseHitLocation`))
      (`self.K2_ExecuteGameplayCue` (struct :`TagName` "GameplayCue.ShockBurst"))
      (`|ExecutionSequence`
        (:`then_0`
          (set `PlayerController.bShowMouseCursor` false (`self.OwnerPlayerController`))
          (`AbilityTask_PlayMontageAndWait.CreatePlayMontageAndWaitProxy` "None" (`self.ElectrocuteMontage`) 1.0 "None" false
            (:`then`
              (`self.K2_HasAuthority`
                (:`True`
                  (`AbilityTask_WaitGameplayEvent.WaitGameplayEvent` (struct :`TagName` "Event.Montage.Electrocute") null true
                    (:`EventReceived`
                      (`self.Shock Loop`)
                      (`self.SpawnBeam`)
                      (bind _returnvalue (`KismetSystemLibrary.K2_SetTimerDelegate` (delegate `DamageAndCost`) (`self.DamageDeltaTime`) true))
                      (set `self.DamageAndCostTimer` _returnvalue))))))))
        (:`then_1`
          (bind (_asynctaskproxy_2 _timeheld) (`AbilityTask_WaitInputRelease.WaitInputRelease` false)
            (:`OnRelease`
              (bind _output_get (set `self.Time Held` _timeheld))
              (if (< _output_get (`self.MinSpellTime`))
                (`self.K2_HasAuthority`
                  (:`True`
                    (`KismetSystemLibrary.Delay` (- (`self.MinSpellTime`) (`self.Time Held`)))
                    (`self.Pre - End Ability` :!label _label)
                    (`self.K2_EndAbility`))
                  (:`False`
                    (`self.Pre - End Ability`)))
                (else
                  (goto _label))))))))))

(event `DamageAndCost`
  (bind _output_get (set `self.Time Held` (+ (stale _output_get) (`self.DamageDeltaTime`))))
  (if (> _output_get (`self.MaxHoldTime`))
    (`self.Pre - End Ability` :!label _label_2)
    (`self.K2_EndAbility`)
    (else
      (bind _returnvalue (`self.K2_CommitAbilityCost` false))
      (if _returnvalue
        (`self.Apply Damage`)
        (else
          (goto _label_2))))))

(event `OnDeath_Event`
  (params (DeadCharacter :type "Actor Object Reference"))
  (`self.Pre - End Ability`)
  (`self.K2_EndAbility`))

(event `self.PrimaryTargetDied`
  (params (DeadActor :type "Actor Object Reference"))
  (`GameplayCueFunctionLibrary.RemoveGameplayCueOnActor` DeadActor (struct :`TagName` "GameplayCue.ShockLoop") (`self.FirstTargetCueParams`))
  (`self.Pre - End Ability`)
  (`self.K2_EndAbility`))

(event `self.AdditionalTargetDied`
  (params (DeadActor :type "Actor Object Reference"))
  (bind (_value _returnvalue) (`BlueprintMapLibrary.Map_Find` (`self.ActorToCueParamsMap`) DeadActor))
  (`KismetArrayLibrary.Array_RemoveItem` (`self.AdditionalTargets`) DeadActor)
  (if _returnvalue
    (`GameplayCueFunctionLibrary.RemoveGameplayCueOnActor` DeadActor (struct :`TagName` "GameplayCue.ShockLoop") _value)))

(event `DelayedEnd`
  (`KismetSystemLibrary.Delay` 0.5)
  (`self.Pre - End Ability`)
  (`self.K2_EndAbility`))

(fn `AddShockLoopCueToTarget`
  (params (TargetActor :type "Actor Object Reference"))
  (bind _targetactor (`local.TargetActor`))
  (bind _returnvalue (`AbilitySystemBlueprintLibrary.MakeGameplayCueParameters` 0.0 0.0 (struct) (struct) (struct) (struct) (struct) (`Actor.K2_GetActorLocation` _targetactor) (0.0 0.0 0.0) null null _targetactor null 1 1 (`Actor.RootComponent` (`self.MouseHitActor`))))
  (`BlueprintMapLibrary.Map_Add` (`self.ActorToCueParamsMap`) (`local.TargetActor`) _returnvalue)
  (`GameplayCueFunctionLibrary.AddGameplayCueOnActor` (`local.TargetActor`) (struct :`TagName` "GameplayCue.ShockLoop") _returnvalue))

(fn `Apply Damage`
  (`self.ApplyDamageToSingleTarget` (`self.MouseHitActor`))
  (for _array_element (`self.AdditionalTargets`)
    (`self.ApplyDamageToSingleTarget` _array_element)))

(fn `ApplyDamageToSingleTarget`
  (params (Target :type "Actor Object Reference"))
  (bind _returnvalue (`self.GetAbilitySystemComponentFromActorInfo`))
  (`/Engine/EditorBlueprintResources/StandardMacros.IsValid` Target
    (:`Is Valid`
      (`AbilitySystemBlueprintLibrary.AssignTagSetByCallerMagnitude` (`AbilitySystemComponent.MakeOutgoingSpec` _returnvalue (`self.DamageEffectClass`) (`KismetMathLibrary.Conv_IntToDouble` (`self.GetAbilityLevel`)) (`AbilitySystemComponent.MakeEffectContext` _returnvalue)) (struct :`TagName` "Damage.Lightning") (`self.GetDamageAtCurrentLevel`))
      (`AuraAbilitySystemLibrary.ApplyDamageEffect` (`self.MakeDamageEffectParamsFromEffectDefaults` (`local.Target`))))))

(fn `EnforceCombatInterface`
  (if (not (`KismetSystemLibrary.DoesImplementInterface` (`self.GetAvatarActorFromActorInfo`) "/Script/Aura.CombatInterface"))
    (`self.K2_EndAbility`)))

(fn `MakeDebuffDamageEffectsParams`
  (params (Target :type "Actor Object Reference"))
  (returns (Params :type "DamageEffectParams Structure"))
  (bind (_returnvalue_worldcontextobject _returnvalue_damagegameplayeffectclass _returnvalue_sourceasc _returnvalue_targetasc _returnvalue_basedamage _returnvalue_abilitylevel _returnvalue_damagetype _returnvalue_debuffchance _returnvalue_debuffdamage _returnvalue_debufffrequency _returnvalue_debuffduration _returnvalue_deathimpulsemagnitudeminmax _returnvalue_deathimpulse _returnvalue_bshouldhitreact) (break `DamageEffectParams` (`self.MakeDamageEffectParamsFromEffectDefaults` Target)))
  (return (make `DamageEffectParams` _returnvalue_worldcontextobject _returnvalue_damagegameplayeffectclass _returnvalue_sourceasc _returnvalue_targetasc 0.0 _returnvalue_abilitylevel _returnvalue_damagetype 100.0 0.0 1.0 (`self.Stun Duration`) _returnvalue_deathimpulsemagnitudeminmax _returnvalue_deathimpulse _returnvalue_bshouldhitreact)))

(fn `Pre - End Ability`
  (bind _mousehitactor (`self.MouseHitActor`))
  (`self.K2_CommitAbilityCooldown` true)
  (set `PlayerController.bShowMouseCursor` true (`self.OwnerPlayerController`))
  (message `CombatInterface.SetInShockLoop` (`self.GetAvatarActorFromActorInfo`) false)
  (`CharacterMovementComponent.SetMovementMode` (`Character.CharacterMovement` (`self.OwnerCharacter`)) "MOVE_Walking" 0)
  (`GameplayCueFunctionLibrary.RemoveGameplayCueOnActor` (`self.Cue Target`) (struct :`TagName` "GameplayCue.ShockLoop") (`self.FirstTargetCueParams`))
  (message `CombatInterface.SetBeingShocked` (`self.Cue Target`) false)
  (if (`KismetSystemLibrary.DoesImplementInterface` _mousehitactor "/Script/Aura.CombatInterface")
    (`self.K2_HasAuthority`
      (:`True`
        (`AuraAbilitySystemLibrary.ApplyDamageEffect` (`self.MakeDebuffDamageEffectsParams` _mousehitactor)))
      (:`False`
        _)))
  (`KismetSystemLibrary.K2_ClearAndInvalidateTimerHandle` (`self.DamageAndCostTimer`))
  (`self.RemoveShockLoopCueFromAdditionalTargets`)
  (`KismetArrayLibrary.Array_Clear` (`self.AdditionalTargets`))
  (`BlueprintMapLibrary.Map_Clear` (`self.ActorToCueParamsMap`))
  (set `self.MouseHitActor` null)
  (set `self.Time Held` 0.0)
  (set `self.Cue Target` null))

(fn `RemoveShockLoopCueFromAdditionalTargets`
  (for _array_element (`self.AdditionalTargets`)
    (bind (_value _returnvalue) (`BlueprintMapLibrary.Map_Find` (`self.ActorToCueParamsMap`) _array_element))
    (if _returnvalue
      (`GameplayCueFunctionLibrary.RemoveGameplayCueOnActor` _array_element (struct :`TagName` "GameplayCue.ShockLoop") _value)
      (message `CombatInterface.SetBeingShocked` _array_element false)
      (`self.K2_HasAuthority`
        (:`True`
          (`AuraAbilitySystemLibrary.ApplyDamageEffect` (`self.MakeDebuffDamageEffectsParams` _array_element)))))))

(fn `Shock Loop`
  (message `CombatInterface.SetInShockLoop` (`self.GetAvatarActorFromActorInfo`) true)
  (`CharacterMovementComponent.DisableMovement` (`Character.CharacterMovement` (`self.OwnerCharacter`))))

(fn `SpawnBeam`
  (locals (`IsFirstHitTargetAnEnemy?` :type Boolean :default false))
  (`self.TraceFirstTarget` (`self.MouseHitLocation`))
  (bind _returnvalue (message `CombatInterface.GetWeapon` (`self.OwnerCharacter`)))
  (set `self.FirstTargetCueParams` (`AbilitySystemBlueprintLibrary.MakeGameplayCueParameters` 0.0 0.0 (struct) (struct) (struct) (struct) (struct) (`self.MouseHitLocation`) (0.0 0.0 0.0) null null (`self.MouseHitActor`) null 1 1 _returnvalue))
  (bind _output_get (set `local.IsFirstHitTargetAnEnemy?` (`KismetSystemLibrary.DoesImplementInterface` (`self.MouseHitActor`) "/Script/Aura.CombatInterface")))
  (bind _output_get_2 (set `self.Cue Target` (select `bool` _output_get :`false` (`self.GetAvatarActorFromActorInfo`) :`true` (`self.MouseHitActor`))))
  (message `CombatInterface.SetBeingShocked` _output_get_2 true)
  (`GameplayCueFunctionLibrary.AddGameplayCueOnActor` _output_get_2 (struct :`TagName` "GameplayCue.ShockLoop") (`self.FirstTargetCueParams`))
  (if (`local.IsFirstHitTargetAnEnemy?`)
    (bind _output_get_3 (set `self.AdditionalTargets` (`self.StoreAdditionalTargets`)))
    (for _array_element _output_get_3
      (`self.AddShockLoopCueToTarget` _array_element)
      (message `CombatInterface.SetBeingShocked` _array_element true))
    (else
      (`self.DelayedEnd`))))