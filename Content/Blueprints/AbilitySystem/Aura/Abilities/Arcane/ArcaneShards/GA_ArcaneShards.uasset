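; Arcane Shards gameplay ability: erupts a series of shards around a point under the mouse, dealing radial damage with outward knockback.
; A magic circle shows until input press, then the ability commits, gets points from a spawned point collection and plays the cast montage.
; The montage event starts a looping timer that fires a gameplay cue and damages nearby live players per shard, up to ability level (capped), then cleans up.
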(event `self.K2_ActivateAbility`
  (bind _returnvalue (`self.K2_CheckAbilityCooldown`))
  (if _returnvalue
    (bind _returnvalue_2 (message `PlayerInterface.ShowTargetingActor` (`self.GetAvatarActorFromActorInfo`) "/Game/Blueprints/AbilitySystem/Aura/Abilities/Arcane/ArcaneShards/BP_MagicCircle.BP_MagicCircle_C" true null (`self.RadialDamageOuterRadius`)))
    (set `self.Targeting Actor` _returnvalue_2)
    (`AbilityTask_WaitInputPress.WaitInputPress` false
      (:`OnPress`
        (bind _returnvalue_3 (`self.K2_CommitAbility`))
        (if _returnvalue_3
          (bind (_asynctaskproxy _data) (`TargetDataUnderMouse.CreateTargetDataUnderMouse`)
            (:`ValidDataHandle`
              (bind (_returnvalue_bblockinghit _returnvalue_binitialoverlap _returnvalue_time _returnvalue_distance _returnvalue_location _returnvalue_impactpoint) (`GameplayStatics.BreakHitResult` (`AbilitySystemBlueprintLibrary.GetHitResultFromTargetData` _data)))
              (bind _output_get (set `self.MouseHitLocation` _returnvalue_impactpoint))
              (bind _returnvalue_4 (`|SpawnActorFromClass` "/Game/Blueprints/AbilitySystem/Aura/Abilities/Arcane/ArcaneShards/BP_PointCollection.BP_PointCollection_C" (`KismetMathLibrary.MakeTransform` _output_get) "AlwaysSpawn" "MultiplyWithRoot" null null))
              (bind _output_get_2 (set `self.PointCollection` _returnvalue_4))
              (set `self.GroundPoints` (`PointCollection.GetGroundPoints` _output_get_2 (`self.MouseHitLocation`) (`self.GetNumShards`) 0.0))
              (message `CombatInterface.SetFacingTarget` (`self.GetAvatarActorFromActorInfo`) (`self.MouseHitLocation`))
              (`AbilityTask_PlayMontageAndWait.CreatePlayMontageAndWaitProxy` "None" "/Game/Assets/Characters/Aura/Animations/Abilities/AM_Cast_ArcaneShards_Short.AM_Cast_ArcaneShards_Short"
                (:`then`
                  (`AbilityTask_WaitGameplayEvent.WaitGameplayEvent` (struct :`TagName` "Event.Montage.ArcaneShards") null
                    (:`EventReceived`
                      (bind _returnvalue_5 (`KismetSystemLibrary.K2_SetTimerDelegate` (delegate `SpawnShard`) (`self.ShardSpawnDeltaTime`) true))
                      (set `self.SpawnShardTimer` _returnvalue_5)
                      (message `PlayerInterface.ShowTargetingActor` (`self.GetAvatarActorFromActorInfo`) null false null 0.0)))))))
          (else
            (`self.K2_EndAbility`)))))
    (else
      (`self.K2_EndAbility`))))

(event `SpawnShard`
  (bind _returnvalue (`self.GetAvatarActorFromActorInfo`))
  (bind _output (`|GetArrayItem` (`self.GroundPoints`) (`self.Count`)))
  ;[0.1279 0.8903 1] Spawn Shard
  (if (< (`self.Count`) (`self.GetNumShards`))
    (bind _output_get (set `self.SpawnLocation` (`SceneComponent.K2_GetComponentLocation` _output)))
    (`self.K2_ExecuteGameplayCueWithParams` (struct :`TagName` "GameplayCue.ArcaneShards") (`AbilitySystemBlueprintLibrary.MakeGameplayCueParameters` 0.0 0.0 (struct) (struct) (struct) (struct) (struct) _output_get (`SceneComponent.GetRightVector` _output)))
    (`/Engine/EditorBlueprintResources/StandardMacros.IncrementInt` (`self.Count`)
      (:`  `
        (bind _outoverlappingactors (`AuraAbilitySystemLibrary.GetLivePlayersWithinRadius` _returnvalue (`|MakeArray` _returnvalue) (`self.RadialDamageOuterRadius`) (`self.SpawnLocation`)))
        (for _array_element _outoverlappingactors
          (bind _returnvalue_2 (- (`Actor.K2_GetActorLocation` _array_element) (`self.SpawnLocation`)))
          (`AuraAbilitySystemLibrary.ApplyDamageEffect` (`self.MakeDamageEffectParamsFromEffectDefaults` _array_element (`self.SpawnLocation`) true _returnvalue_2 true _returnvalue_2)))))
    (else
      ;[1 1 1] Ability End
      (set `self.Count` 0)
      (`KismetArrayLibrary.Array_Clear` (`self.GroundPoints`))
      (`KismetSystemLibrary.K2_ClearAndInvalidateTimerHandle` (`self.SpawnShardTimer`))
      (`Actor.K2_DestroyActor` (`self.PointCollection`))
      (bind _targeting_actor (`self.Targeting Actor`)
        (:`then`
          (`Actor.K2_DestroyActor` _targeting_actor))
        (:`else`
          _))
      (`self.K2_EndAbility`))))

(event `self.K2_OnEndAbility`
  (params (bWasCancelled :type Boolean)))

(fn `GetNumShards`
  (returns (NumShards :type Integer))
  (return (`KismetMathLibrary.Min` (`self.GetAbilityLevel`) (`self.MaxNumShards`))))