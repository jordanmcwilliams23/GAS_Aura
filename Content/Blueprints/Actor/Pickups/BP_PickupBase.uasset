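; Base pickup actor that pops into the world with a jump animation and sound feedback; it holds no collection logic.
; On BeginPlay it picks a random apex height, then a timeline drives scale and a vertical offset from the spawn location through CalculateHeight.
; A separate timed delay triggers the ground impact sound rather than collision detection.
; Spawn plays its own sound, and any destruction plays the consumed sound.
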(event `self.ReceiveBeginPlay`
  (bind (_spawnapexminmax_x _spawnapexminmax_y) (`KismetMathLibrary.BreakVector2D` (`self.SpawnApexMinMax`)))
  (`GameplayStatics.PlaySoundAtLocation` (`self.SpawnSound`) (`self.K2_GetActorLocation`) (struct) 1.0 1.0 0.0 null null null null)
  (set `self.StartingLocation` (`self.K2_GetActorLocation`))
  (set `self.Spawn Apex` (`KismetMathLibrary.RandomFloatInRange` _spawnapexminmax_x _spawnapexminmax_y))
  (`|ExecutionSequence`
    (:`then_0`
      (bind (_direction _height _scale) (`Timeline|JumpTimeline`)
        (:`Update`
          (`self.K2_SetActorLocation` (`self.CalculateHeight` _height))
          (`self.SetActorScale3D` (`KismetMathLibrary.MakeVector` _scale _scale _scale)))))
    (:`then_1`
      (`KismetSystemLibrary.Delay` (`self.TimeTilHitGround`))
      (`GameplayStatics.PlaySoundAtLocation` (`self.GroundImpactSound`) (`self.K2_GetActorLocation`) (struct) 1.0 1.0 0.0 null null null null))))

(event `self.ReceiveDestroyed`
  (`GameplayStatics.PlaySoundAtLocation` (`self.ConsumedSound`) (`self.K2_GetActorLocation`) (struct) 1.0 1.0 0.0 null null null null))

(fn `CalculateHeight`
  (params (A :type "Float (double-precision)"))
  (returns (ReturnValue :type "Vector Structure"))
  (return (+ (`KismetMathLibrary.MakeVector` 0.0 0.0 (* A (`self.Spawn Apex`))) (`self.StartingLocation`))))

(fn `UserConstructionScript`)