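; Checkpoint beacon that lights up with a chime when an actor implementing PlayerInterface enters its sphere.
; The overlap sets Activated and creates a dynamic material instance, whose Glow parameter a timeline drives, scaled by GlowMultiplier.
; On load, LoadActor restores full glow if Activated, and ShouldLoadTransform returns false to skip transform loading.
; Overlap has no Activated check, so the chime replays on each entry.
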(event `SaveInterface.LoadActor`
  ;[1 1 1] Load Actor
  (if (`self.Activated?`)
    (bind _returnvalue (`PrimitiveComponent.CreateDynamicMaterialInstance` (`self.BeaconMesh`) 0 null "None"))
    (bind _output_get (set `self.DMI_Beacon` _returnvalue))
    (`PrimitiveComponent.SetMaterial` (`self.BeaconMesh`) 0 _output_get)
    (`MaterialInstanceDynamic.SetScalarParameterValue` _output_get "Glow" (`self.GlowMultiplier`))))

(event `self.Sphere.OnComponentBeginOverlap`
  (params (OverlappedComponent :type "PrimitiveComponent Object Reference") (OtherActor :type "Actor Object Reference") (OtherComp :type "PrimitiveComponent Object Reference") (OtherBodyIndex :type Integer) (bFromSweep :type Boolean) (SweepResult :type "HitResult Structure (by ref)"))
  (if (`KismetSystemLibrary.DoesImplementInterface` OtherActor "/Script/Aura.PlayerInterface")
    (set `self.Activated?` true)
    (`GameplayStatics.PlaySoundAtLocation` "/Game/Assets/Sounds/Misc/MysticalChime_Cue.MysticalChime_Cue" (`self.K2_GetActorLocation`) (struct) 1.0 1.0 0.0 "/Game/Assets/Sounds/Attenuations/ATT_Torch.ATT_Torch" null null null)
    (bind _returnvalue (`PrimitiveComponent.CreateDynamicMaterialInstance` (`self.BeaconMesh`) 0 null "None"))
    (bind _output_get (set `self.DMI_Beacon` _returnvalue))
    (`PrimitiveComponent.SetMaterial` (`self.BeaconMesh`) 0 _output_get)
    (bind (_direction _beacontrack) (`Timeline|Beacon Timeline`)
      (:`Update`
        (`MaterialInstanceDynamic.SetScalarParameterValue` _output_get "Glow" (* _beacontrack (`self.GlowMultiplier`)))))))

(fn `ShouldLoadTransform`
  (returns (ReturnValue :type Boolean))
  (return false))

(fn `UserConstructionScript`)