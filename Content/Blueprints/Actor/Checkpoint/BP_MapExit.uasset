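; BP_MapExit is a map exit actor that lights up when highlighted.
; The highlight and unhighlight events call the parent versions, then show or hide two point lights.
; GetMoveToLocation returns the zero vector, and the construction script is empty.
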(event `HighlightInterface.HighlightActor`
  (`parent.HighlightActor`)
  (`SceneComponent.SetVisibility` (`self.PointLight`) true false)
  (`SceneComponent.SetVisibility` (`self.PointLight1`) true false))

(event `HighlightInterface.UnhighlightActor`
  (`parent.UnhighlightActor`)
  (`SceneComponent.SetVisibility` (`self.PointLight`) false false)
  (`SceneComponent.SetVisibility` (`self.PointLight1`) false false))

(fn `GetMoveToLocation`
  (returns (ReturnValue :type "Vector Structure"))
  (return (0.0 0.0 0.0)))

(fn `UserConstructionScript`)