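; BP_DungeonStair is a dungeon stair actor, filed with the checkpoint actors, that lights up when highlighted.
; It extends the parent's HighlightActor and UnhighlightActor events, calling the parent first and then showing or hiding its two point lights.
; The construction script only calls the parent, and this graph adds no other stair or checkpoint logic.
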(event `HighlightInterface.HighlightActor`
  (`parent.HighlightActor`)
  (`SceneComponent.SetVisibility` (`self.PointLight`) true false)
  (`SceneComponent.SetVisibility` (`self.PointLight1`) true false))

(event `HighlightInterface.UnhighlightActor`
  (`parent.UnhighlightActor`)
  (`SceneComponent.SetVisibility` (`self.PointLight`) false false)
  (`SceneComponent.SetVisibility` (`self.PointLight1`) false false))

(fn `UserConstructionScript`
  (`parent.UserConstructionScript`))