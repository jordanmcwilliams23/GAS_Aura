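; BP_Random_ore is an ore prop actor for the crystal cave that varies its look per placed instance.
; Its construction script loops over four static mesh components, giving each a random mesh from the RandomMesh array and a random yaw rotation.
; Randomness is unseeded, so the look re-rolls whenever construction reruns, and the event graph holds no active logic.
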(fn `UserConstructionScript`
  ;[1 1 1] Randomize Mesh
  (for _array_element (`|MakeArray` (`self.StaticMesh`) (`self.StaticMesh2`) (`self.StaticMesh3`) (`self.StaticMesh4`))
    (`StaticMeshComponent.SetStaticMesh` _array_element (`KismetArrayLibrary.Array_Random` (`self.RandomMesh`)))
    (`SceneComponent.K2_SetRelativeRotation` _array_element (`KismetMathLibrary.MakeRotator` 0.0 0.0 (`KismetMathLibrary.RandomFloatInRange` 0.0 360.0)) false false)))